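; Blueprint utility library that generates and manipulates spatial point and transform arrays for procedural shapes, with millimetre unit conversion.
; Normalized line steps feed a circle function to build arcs of transforms, oriented along finite-difference tangents.
; Arcs become circles, offset U-bends and rounded trapezoid profiles through helpers that transform, slice, merge and flatten arrays to 2D.
; Some helpers print debug output, mostly array lengths.
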(fn Line1D
  (params (steps :type Integer) (closed :type Boolean))
  (bind _returnvalue (- steps 1))
  (for _index (range 0 _returnvalue)
    (Utilities|Array|SetArrayElem (LocalVariables|Get_line) _index (/ (Math|Conversions|ToFloat(Integer) _index) (Math|Integer|SelectInt _returnvalue steps closed)) true))
  (return (LocalVariables|Get_line)))

(fn Arc4D
  (params (radius_mm :type Float%20%28double-precision%29) (steps :type Integer) (filled_norm :type Float%20%28double-precision%29) (offset_norm :type Float%20%28double-precision%29))
  (LocalVariables|Setmm_radius radius_mm)
  (Utilities|Array|Resize (LocalVariables|Getarc_spots) steps)
  (bind _line (shape|Line1D steps true))
  (for (_array_element _array_index) _line
    (Utilities|Array|SetArrayElem (LocalVariables|Getarc_spots) _array_index (CallFunction|CircleTrans (LocalVariables|Getmm_radius) (+ (* _array_element filled_norm) offset_norm))))
  (return (LocalVariables|Getarc_spots)))

(fn Tupi
  (params (progress :type Float%20%28double-precision%29))
  (return (* progress (Math|Float|MultiplybyPi 2.0))))

(fn VtoMm
  (params (ueu :type Vector))
  (return (* ueu (Utilities|MmConverionRate))))

(fn CirclePos
  (params (pos_1d :type Float%20%28double-precision%29))
  (bind _redians (CallFunction|Tupi pos_1d))
  (return (size|VtoMm (Math|Vector|MakeVector (Math|Trig|Cos(Radians) _redians) (Math|Trig|Sin(Radians) _redians) 0.0))))

(fn CircleTrans
  (params (radius_mm :type Float%20%28double-precision%29) (pos_1d :type Float%20%28double-precision%29))
  (bind _v_mm (CallFunction|CirclePos pos_1d))
  (return (Math|Transform|MakeTransform (* radius_mm _v_mm) (Math|Rotator|MakeRotfromX (- (CallFunction|CirclePos (+ pos_1d 0.0001)) _v_mm)))))

(fn StoMm
  (params (ueu :type Float%20%28double-precision%29))
  (return (* ueu (Utilities|MmConverionRate))))

(fn Half
  (params (whole :type Float%20%28double-precision%29))
  (return (* whole 0.5)))

(fn TXT
  (params (spots :type Array%20of%20Transforms) (operation :type Transform))
  (Utilities|Array|Resize (LocalVariables|Getnew_spots) (Utilities|Array|Length spots))
  (for (_array_element _array_index) spots
    (Utilities|Array|SetArrayElem (LocalVariables|Getnew_spots) _array_index (Math|Transform|ComposeTransforms operation _array_element)))
  (return (LocalVariables|Getnew_spots)))

(fn VXT
  (params (Array :type Array%20of%20Vectors) (T :type Transform%20%28by%20ref%29))
  (Utilities|Array|Resize (LocalVariables|Getarray_trasformed) (Utilities|Array|Length Array))
  (for (_array_element _array_index) Array
    (Utilities|Array|SetArrayElem (LocalVariables|Getarray_trasformed) _array_index (Math|Transform|TransformLocation T _array_element)))
  (return (LocalVariables|Getarray_trasformed)))

(fn VtoP
  (params (array_3d :type Array%20of%20Vectors))
  (Utilities|Array|Resize (LocalVariables|Getarray_cache) (Utilities|Array|Length array_3d))
  (for (_array_element _array_index) array_3d
    (Utilities|Array|SetArrayElem (LocalVariables|Getarray_cache) _array_index (Math|Vector2D|MakeVector2D (.x _array_element) (.y _array_element))))
  (return (LocalVariables|Getarray_cache)))

(fn RoundTrapez2D
  (params (radius_mm :type Float%20%28double-precision%29) (steps :type Integer))
  (LocalVariables|Setradius_mm_ radius_mm)
  (LocalVariables|Setlocal_res steps)
  (bind _arc_spots_ (shape|Arc4D (LocalVariables|Getradius_mm_) (+ (LocalVariables|Getlocal_res) 1) 1.0 0.0))
  (bind _outputpin (ops|VXT (CallFunction|SubSelect (ops|TtoV _arc_spots_) (* (Class|KismetSystemLibrary|MakeLiteralInteger 2) (/ (LocalVariables|Getlocal_res) 4)) (+ (+ (* (Class|KismetSystemLibrary|MakeLiteralInteger 2) (/ (LocalVariables|Getlocal_res) 4)) (/ (LocalVariables|Getlocal_res) 4)) 1)) (Math|Transform|MakeTransform (size|VtoMm (Math|Vector|MakeVector (* (LocalVariables|Getradius_mm_) 2.0) 0.0 0.0)) "0, 0, 0" "1.000000,1.000000,1.000000")))
  (log|VLenLog _outputpin "first_half")
  (bind _outputpin_2 (ops|VXT (CallFunction|SubSelect (ops|TtoV _arc_spots_) (* (Class|KismetSystemLibrary|MakeLiteralInteger 3) (/ (LocalVariables|Getlocal_res) 4)) (+ (+ (* (Class|KismetSystemLibrary|MakeLiteralInteger 3) (/ (LocalVariables|Getlocal_res) 4)) (/ (LocalVariables|Getlocal_res) 4)) 1)) (Math|Transform|MakeTransform (size|VtoMm (Math|Vector|MakeVector (MathSimple|SNeg (* (LocalVariables|Getradius_mm_) 2.0)) 0.0 0.0)) "0, 0, 0" "1.000000,1.000000,1.000000")))
  (log|VLenLog _outputpin_2 "last_half")
  (bind _outputpin_3 (array|Merge3D _outputpin _outputpin_2))
  (log|VLenLog _outputpin_3 "mergerd")
  (bind _array_2d (ops|VtoP _outputpin_3))
  (Utilities|Array|Reverse _array_2d)
  (return _array_2d))

(fn SubSelect
  (params (v_from :type Array%20of%20Vectors) (from :type Integer) (to :type Integer))
  (LocalVariables|Setfirst_idx from)
  (Utilities|Array|Resize (LocalVariables|Getsub_selection) (- to (LocalVariables|Getfirst_idx)))
  (for _index (range (LocalVariables|Getfirst_idx) (- to 1))
    (Utilities|Array|SetArrayElem (LocalVariables|Getsub_selection) (- _index (LocalVariables|Getfirst_idx)) (Utilities|Array|Get(acopy) v_from _index)))
  (return (LocalVariables|Getsub_selection)))

(fn TtoV
  (params (t :type Array%20of%20Transforms))
  (Utilities|Array|Resize (LocalVariables|Getpositions) (Utilities|Array|Length t))
  (for (_array_element _array_index) t
    (Utilities|Array|SetArrayElem (LocalVariables|Getpositions) _array_index (.location _array_element)))
  (return (LocalVariables|Getpositions)))

(fn Circle2D
  (params (radius_mm :type Float%20%28double-precision%29) (shape :type Integer))
  (bind _arc_spots_ (shape|Arc4D radius_mm shape (/ (Math|Conversions|ToFloat(Integer) (- shape 1)) (Math|Conversions|ToFloat(Integer) shape)) 0.0))
  (bind _array_2d (ops|VtoP (ops|TtoV _arc_spots_)))
  (return _array_2d))

(fn SNeg
  (params (s :type Float%20%28double-precision%29))
  (return (* s -1.0)))

(fn Merge3D
  (params (a :type Array%20of%20Vectors) (b :type Array%20of%20Vectors))
  (for _array_element a
    (Utilities|Array|Add (LocalVariables|Getcombined) _array_element))
  (for _array_element_2 b
    (Utilities|Array|Add (LocalVariables|Getcombined) _array_element_2))
  (return (LocalVariables|Getcombined)))

(fn VLenLog
  (params (InputPin :type Array%20of%20Vectors) (name_tag :type String))
  (Development|PrintString 0 (Utilities|String|Append "+++ v_len_log (" name_tag "): " (Utilities|String|ToString(Integer) (Utilities|Array|Length InputPin))))
  (return))

(fn VHalf
  (params (path_whole :type Array%20of%20Vector%202D%20Structures))
  (bind _output_get (LocalVariables|Setpath path_whole))
  (bind _output_get_2 (LocalVariables|Sethalf_size (/ (Utilities|Array|Length _output_get) 2)))
  (Utilities|Array|Resize (LocalVariables|Gethalf_path) _output_get_2)
  (for _index (range 0 (- (LocalVariables|Gethalf_size) 1))
    (Utilities|Array|SetArrayElem (LocalVariables|Gethalf_path) _index (Utilities|Array|Get(acopy) (LocalVariables|Getpath) _index))
    (Development|PrintString 0 "dupa"))
  (return (LocalVariables|Gethalf_path)))

(fn PLenLog
  (params (InputPin :type Array%20of%20Vector%202D%20Structures) (name_tag :type String) (__WorldContext :type Object%20Object%20Reference))
  (Development|PrintString 0 (Utilities|String|Append "+++ v_len_log (" name_tag "): " (Utilities|String|ToString(Integer) (Utilities|Array|Length InputPin))))
  (return))

(fn U4D
  (params (radius_mm :type Float%20%28double-precision%29) (steps :type Integer) (arms_len_mm :type Float%20%28double-precision%29))
  (bind _arc_spots_ (shape|Arc4D radius_mm steps 0.5 0.0))
  (bind _t (ops|TXT _arc_spots_ (Math|Transform|MakeTransform (size|VtoMm (Math|Vector|MakeVector (MathSimple|Half arms_len_mm) 0.0 0.0)) "0, 0, 0" "1.000000,1.000000,1.000000")))
  (return _t))

(fn Merge4D
  (params (a :type Array%20of%20Transforms) (b :type Array%20of%20Transforms))
  (for _array_element a
    (Utilities|Array|Add (LocalVariables|Getcombined) _array_element))
  (for _array_element_2 b
    (Utilities|Array|Add (LocalVariables|Getcombined) _array_element_2))
  (return (LocalVariables|Getcombined)))