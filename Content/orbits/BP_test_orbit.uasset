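; Test orbit actor that moves a referenced Body actor along a spline path in a repeating loop.
; Each Tick advances Time by TimeFlow, resets it to zero past 1, and sets the Body's location from the spline's world transform at that time.
; Disconnected leftovers hold a variant that also applies rotation and a construction-script loop that generates circular spline points, so neither runs.
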(event EventBeginPlay)

(event Collision|EventActorBeginOverlap
  (params (OtherActor :type Actor%20Object%20Reference)))

(event EventTick
  (params (DeltaSeconds :type Float%20%28single-precision%29))
  (Utilities|FlowControl|Sequence
    (:then_0
      (Variables|Default|Settime (Math|Float|SelectFloat 0.0 (+ (Variables|Default|Gettime) (* (Variables|Default|Gettime_flow) DeltaSeconds)) (> (+ (Variables|Default|Gettime) (* (Variables|Default|Gettime_flow) DeltaSeconds)) 1.0))))
    (:then_1
      (Utilities|IsValid (Variables|Default|Getbody)
        (:Is%20Valid
          (Transformation|SetActorLocation (Variables|Default|Getbody) (.Location (Math|Transform|BreakTransform (Spline|GetTransformatTime (Variables|Default|GetSpline) (Variables|Default|Gettime) "World" false false))) false false))))))

(fn ConstructionScript)