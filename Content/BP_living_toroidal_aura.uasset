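; Toroidal aura actor that arranges BP_space_time_point child actors in a ring and spins it with an organically varying speed.
; Construction script spaces ArmsNum points evenly in the local YZ plane at MRadius, scaled by 100, and sets the dynamic mesh's roll to preview the swirl.
; Tick rolls the actor at a speed interpolated between random samples refreshed each second.
; ChangeMaterial forwards a material to PutSomeMaterial.
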(event EventBeginPlay
  (|CallParentFunction) ; This node is disabled and will not be called.\nDrag off pins to build functionality.
)

(event Collision|EventActorBeginOverlap
  (params (OtherActor :type Actor%20Object%20Reference))
  (|CallParentFunction OtherActor) ; This node is disabled and will not be called.\nDrag off pins to build functionality.
)

(event EventTick
  (params (DeltaSeconds :type Float%20%28single-precision%29))
  (|CallParentFunction DeltaSeconds)
  (Utilities|FlowControl|Sequence
    (:then_0
      ;[0 0 0] Comment
      (Variables|Default|Settimer (+ DeltaSeconds (Variables|Default|Gettimer)))
      (if (not (< (Variables|Default|Gettimer) 1.0))
        (Variables|Default|Settimer (- (Variables|Default|Gettimer) 1.0))
        ;[0 0 0] future_sample
        (Variables|Default|Setlast_speed (Variables|Default|Getnext_speed))
        (Variables|Default|Setnext_speed (* (.degrees (CallFunction|RandomRot)) 2.0))))
    (:then_1
      ;[0 0 0] update rotation
      (Transformation|AddActorLocalRotation (Math|Rotator|MakeRotator (* DeltaSeconds (Math|Float|Lerp (Variables|Default|Getlast_speed) (Variables|Default|Getnext_speed) (Variables|Default|Gettimer))) 0.0 0.0) false false))))

(fn ConstructionScript
  (|CallParentFunction)
  (Variables|Default|Setradius (* (Variables|Default|Getm_radius) 1e+02))
  (Utilities|FlowControl|Sequence
    (:then_0
      ;[0 0 0] swirl_previrew
      (Transformation|SetRelativeRotation (Variables|Default|GetDynamicMeshComponent) (Math|Rotator|MakeRotator (Variables|Default|Getswirle_angle) 0.0 0.0) false false))
    (:then_1
      ;[0 0 0] radial_patern
      (for _index (range 0 (- (Variables|Default|Getarms_num) 1))
        ;;[0 0 0] creatin_space_time_points
        (bind _returnvalue (AddComponent|AddChildActorComponent false (Math|Transform|MakeTransform (* (Math|Vector|MakeVector 0.0 (Math|Trig|Cos(Radians) (* (/ (Math|Conversions|ToFloat(Integer) _index) (Variables|Default|Getarms_num)) (* (Math|Trig|GetPI) 2.0))) (Math|Trig|Sin(Radians) (* (/ (Math|Conversions|ToFloat(Integer) _index) (Variables|Default|Getarms_num)) (* (Math|Trig|GetPI) 2.0)))) (Variables|Default|Getradius)) "0, 0, 0" "1.000000,1.000000,1.000000")))
        (ChildActorComponent|SetChildActorClass _returnvalue "/cubes_of_time/BP_space_time_point.BP_space_time_point_C")))))

(fn RandomRot
  (bind _returnvalue (Math|Random|RandomFloat))
  (bind _returnvalue_2 (* _returnvalue 2.0))
  (bind _returnvalue_3 (- _returnvalue_2 1.0))
  (return (* _returnvalue_3 1.8e+02) (Math|Float|MultiplybyPi _returnvalue_3)))

(fn ChangeMaterial
  (params (material :type Material%20Interface%20Object%20Reference))
  (Default|PutSomeMaterial self material))