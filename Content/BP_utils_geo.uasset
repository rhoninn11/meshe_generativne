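; Geometry Script helper functions that procedurally build millimetre-sized primitives: boxes, cylinders, circle sweeps, hollow tubes and round-ended sticks (patyk).
; Builders draw compute meshes from a geometry actor, with optional allocation in some.
; The tube sweeps a circle along a curve-scaled line, then subtracts a shrunken copy to hollow it.
; The stick boolean-unions cylinders at transform spots with a connecting box, optionally centred symmetrically.
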(fn MeshOpsInstances
  (params (mesh_dst :type Dynamic%20Mesh%20Object%20Reference) (mesh_to_spawn :type Dynamic%20Mesh%20Object%20Reference) (spots :type Array%20of%20Transforms))
  (LocalVariables|Setmesh_final mesh_dst)
  (LocalVariables|Setmesh_instance mesh_to_spawn)
  (for _array_element spots
    (GeometryScript|Booleans|ApplyMeshBoolean :TargetMesh (LocalVariables|Getmesh_final) :ToolMesh (LocalVariables|Getmesh_instance) :ToolTransform _array_element :Operation "Union" :Debug 0))
  (return (LocalVariables|Getmesh_final)))

(fn GeoTube
  (params (geo_actor :type Dynamic%20Mesh%20Actor%20Object%20Reference) (_mesh_dst :type Dynamic%20Mesh%20Object%20Reference) (shape :type Curve%20Float%20Object%20Reference) (porar_param :type S%20Polar%20Size%20Structure))
  (bind _returnvalue (Math|Float|MakeLiteralFloat 0.8))
  (LocalVariables|Setfn_source geo_actor)
  (LocalVariables|Setfinal_mesh _mesh_dst)
  (LocalVariables|Setobwiednia shape)
  (LocalVariables|Setpolar porar_param)
  ;[0 0 0] transformed line
  (Utilities|FlowControl|Sequence
    (:then_0
      (bind _line_4d_ (CallFunction|Line4D (.len_mm (LocalVariables|Getpolar)) (.steps_along (LocalVariables|Getpolar)))))
    (:then_1
      (bind _line (CallFunction|Line1D (.steps_along (LocalVariables|Getpolar)) true false))
      (bind _sampled_curve (CallFunction|SampleCurve _line (LocalVariables|Getobwiednia)))
      (bind _spots (CallFunction|SarrtoTarr _sampled_curve))
      (bind _t (CallFunction|TarrXTarr _line_4d_ _spots))
      ;[0 0 0] circle
      (bind _array_2d (CallFunction|Circle2D (.radius_mm (LocalVariables|Getpolar)) (.steps_around (LocalVariables|Getpolar))))
      ;[0 0 0] cylinder
      (bind _returnvalue_2 (DynamicMeshActor|AllocateComputeMesh (LocalVariables|Getfn_source)))
      (bind _returnvalue_3 (Class|GeometryScriptLibraryMeshPrimitiveFunctions|AppendSweepPolygon :TargetMesh _returnvalue_2 :PolygonVertices _array_2d :SweepPath _t :Debug 0))
      ;[0 0 0] tube
      ;;[0 0 0] smaller
      (bind _returnvalue_4 (DynamicMeshActor|AllocateComputeMesh (LocalVariables|Getfn_source)))
      (bind _copytomeshout (GeometryScript|Decomposition|CopyMeshtoMesh _returnvalue_3 _returnvalue_4 0))
      (bind _returnvalue_5 (Class|GeometryScriptLibraryMeshTransformFunctions|ScaleMesh _copytomeshout (Math|Vector|MakeVector 1.0 _returnvalue _returnvalue) "0.000000,0.000000,0.000000" true 0))
      (bind _returnvalue_6 (GeometryScript|Booleans|ApplyMeshBoolean :TargetMesh _returnvalue_3 :ToolMesh _returnvalue_5 :Operation "Subtract" :Debug 0))
      (bind _returnvalue_7 (GeometryScript|MeshEdits|AppendMesh :TargetMesh (LocalVariables|Getfinal_mesh) :AppendMesh _returnvalue_6 :AppendOptions "(CombineMode=EnableAllMatching)" :Debug 0))
      (return _returnvalue_7))))

(fn GeoCircleAlong
  (params (geo_actor :type Dynamic%20Mesh%20Actor%20Object%20Reference) (_mesh_dst :type Dynamic%20Mesh%20Object%20Reference) (polar_param :type S%20Polar%20Size%20Structure) (_sweep_along :type Array%20of%20Transforms))
  (LocalVariables|Setfn_source geo_actor)
  (LocalVariables|Setfinal_mesh _mesh_dst)
  (LocalVariables|Setpolar polar_param)
  ;[0 0 0] circle
  (bind _array_2d (CallFunction|Circle2D (.radius_mm (LocalVariables|Getpolar)) (.steps_around (LocalVariables|Getpolar))))
  ;[0 0 0] cylinder
  (bind _returnvalue (DynamicMeshActor|AllocateComputeMesh (LocalVariables|Getfn_source)))
  (bind _returnvalue_2 (Class|GeometryScriptLibraryMeshPrimitiveFunctions|AppendSweepPolygon :TargetMesh _returnvalue :PolygonVertices _array_2d :SweepPath _sweep_along :Debug 0))
  (return _returnvalue_2))

(fn GeoCylin
  (params (lib :type Dynamic%20Mesh%20Actor%20Object%20Reference) (mesh_dst :type Dynamic%20Mesh%20Object%20Reference) (_origin :type EGeometryScriptPrimitiveOriginMode%20Enum :default "Center") (size :type S%20Polar%20Size%20Structure) (alloc :type Boolean))
  (LocalVariables|Setfns lib)
  (LocalVariables|Setfinal_mesh mesh_dst)
  (LocalVariables|Setorigin _origin)
  (LocalVariables|Setpolar size)
  (if alloc
    (bind _returnvalue (DynamicMeshActor|AllocateComputeMesh (LocalVariables|Getfns)))
    (LocalVariables|Setfinal_mesh _returnvalue))
  (bind _returnvalue_2 (GeometryScript|Primitives|AppendCylinder :TargetMesh (LocalVariables|Getfinal_mesh) :Radius (CallFunction|StoMm (.radius_mm (LocalVariables|Getpolar))) :Height (CallFunction|StoMm (.len_mm (LocalVariables|Getpolar))) :RadialSteps (.steps_around (LocalVariables|Getpolar)) :Origin (LocalVariables|Getorigin) :Debug 0))
  (return _returnvalue_2))

(fn GeoBox
  (params (lib :type Dynamic%20Mesh%20Actor%20Object%20Reference) (mesh_dst :type Dynamic%20Mesh%20Object%20Reference) (_origin :type EGeometryScriptPrimitiveOriginMode%20Enum :default "Center") (size_mm :type Vector) (alloc :type Boolean) (__WorldContext :type Object%20Object%20Reference))
  (LocalVariables|Setfns lib)
  (LocalVariables|Setfinal_mesh mesh_dst)
  (LocalVariables|Setorigin _origin)
  (LocalVariables|Setbox_size size_mm)
  (if alloc
    (bind _returnvalue (DynamicMeshActor|AllocateComputeMesh (LocalVariables|Getfns)))
    (LocalVariables|Setfinal_mesh _returnvalue))
  (bind _returnvalue_2 (Class|GeometryScriptLibraryMeshPrimitiveFunctions|AppendBox :TargetMesh (LocalVariables|Getfinal_mesh) :DimensionX (.x (CallFunction|VtoMm (LocalVariables|Getbox_size))) :DimensionY (.y (CallFunction|VtoMm (LocalVariables|Getbox_size))) :DimensionZ (.z (CallFunction|VtoMm (LocalVariables|Getbox_size))) :Origin (LocalVariables|Getorigin) :Debug 0))
  (return _returnvalue_2))

(fn GeoPatyk
  (params (lib :type GBP%20Parametric%20Modeling%20Object%20Reference) (mesh_dst :type Dynamic%20Mesh%20Object%20Reference) (alloc :type Boolean) (is_symetric :type Boolean) (stick_param :type S%20Patyk%20Structure))
  (bind (_mesh_out_ _fns_) (CallFunction|GeoEmpty lib mesh_dst alloc))
  (LocalVariables|Setmesh_final _mesh_out_)
  (LocalVariables|Setfns _fns_)
  (LocalVariables|Setsymetry is_symetric)
  (LocalVariables|Setstick_size stick_param)
  (Utilities|FlowControl|Sequence
    (:then_0
      ;[0 0 0] side_discs
      (bind _mesh_out (BuildingBlocks|GeoCylin (LocalVariables|Getfns) 0 "Center" (Utilities|Struct|MakeS_polar_size (.depth_mm (LocalVariables|Getstick_size)) (CallFunction|DtoR (.width_mm (LocalVariables|Getstick_size))) 0 60) true))
      (bind _line (CallFunction|Line1D 2 true (LocalVariables|Getsymetry)))
      (bind _as_vectors (CallFunction|SarrXV _line (Math|Vector|MakeVector (CallFunction|StoMm (.core_len_mm (LocalVariables|Getstick_size))) 0.0 0.0)))
      (operations|MeshOpsInstances (LocalVariables|Getmesh_final) _mesh_out (CallFunction|VarrtoTarr _as_vectors)))
    (:then_1
      ;[0 0 0] filled_with_bar
      (bind _mesh_out_2 (BuildingBlocks|GeoBox (LocalVariables|Getfns) 0 "Center" (Math|Vector|MakeVector (.core_len_mm (LocalVariables|Getstick_size)) (.width_mm (LocalVariables|Getstick_size)) (.depth_mm (LocalVariables|Getstick_size))) true))
      (bind _returnvalue (Class|GeometryScriptLibraryMeshTransformFunctions|TranslateMesh _mesh_out_2 (Math|Vector|MakeVector (Math|Float|SelectFloat 0.0 (CallFunction|StoMm (CallFunction|Half (.core_len_mm (LocalVariables|Getstick_size)))) (LocalVariables|Getsymetry)) 0.0 0.0) 0))
      (GeometryScript|Booleans|ApplyMeshBoolean :TargetMesh (LocalVariables|Getmesh_final) :ToolMesh _returnvalue :Operation "Union" :Debug 0))
    (:then_2
      (return (LocalVariables|Getmesh_final)))))

(fn GeoEmpty
  (params (fns :type GBP%20Parametric%20Modeling%20Object%20Reference) (mesh_final :type Dynamic%20Mesh%20Object%20Reference) (new :type Boolean))
  (LocalVariables|Setmesh_final_ mesh_final)
  (if new
    (bind _returnvalue (DynamicMeshActor|AllocateComputeMesh fns))
    (LocalVariables|Setmesh_final_ _returnvalue))
  (return (LocalVariables|Getmesh_final_) fns))