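; BP_Exporter copies the mesh of a referenced Dynamic Mesh Actor into a static mesh asset, rescaled for use in Blender.
; Its export event copies the geometry into a temporary compute mesh, scales it by ScaleToBlender divided by the actor's MmConversionRate, and writes it to AssetToExportTo.
; Working on the copy leaves the source mesh untouched, and all compute meshes are released afterwards.
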(event Custom|export
  (bind _dynamic_mesh_actor (Variables|Default|Getdynamic_mesh_actor))
  (Utilities|IsValid _dynamic_mesh_actor
    (:Is%20Valid
      (bind _returnvalue (DynamicMeshComponent|GetDynamicMesh (Variables|/Script/GeometryFramework.DynamicMeshActor|GetDynamicMeshComponent _dynamic_mesh_actor)))
      (bind _returnvalue_2 (DynamicMeshActor|AllocateComputeMesh))
      (bind _copytomeshout (GeometryScript|Decomposition|CopyMeshtoMesh _returnvalue _returnvalue_2 0))
      (bind _returnvalue_3 (Class|GeometryScriptLibraryMeshTransformFunctions|ScaleMesh _copytomeshout (Math|Conversions|ToVector(Float) (/ (Variables|Default|Getscale_to_blender) (Variables|/generaive_mesh/patyczkowe/GBP_parametric_modeling.GBP_parametric_modeling_C|Getmm_conversion_rate _dynamic_mesh_actor))) "0.000000,0.000000,0.000000" true 0))
      (GeometryScript|StaticMesh|CopyMeshtoStaticMesh :FromDynamicMesh _returnvalue_3 :ToStaticMeshAsset (Variables|Default|Getasset_to_export_to) :Debug 0
        (:Failure
          _)
        (:Success
          _))
      (DynamicMeshActor|ReleaseAllComputeMeshes))))

(event EventBeginPlay)

(event Collision|EventActorBeginOverlap
  (params (OtherActor :type Actor%20Object%20Reference)))

(event EventTick
  (params (DeltaSeconds :type Float%20%28single-precision%29)))

(fn ConstructionScript)